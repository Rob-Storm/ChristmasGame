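; Dialogue manager that runs a conversation from an array of dialogue lines in WBP_DialogueUI, firing start and end dispatchers.
; DialogueStart appends a placeholder LastLine entry as an end sentinel, creates the widget, disables player movement and switches to UI-only input.
; DialogueContinue pushes each line to the widget until it hits the sentinel, then calls DialogueEnd to restore control.
; Fixed delays around intro and outro animations time continue input and widget removal.
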(event Custom|DialogueStart
  (params (DialogueLines :type Array%20of%20Dialogue%20Line%20Structures))
  (bind _returnvalue (Game|GetPlayerController 0))
  (Default|CallOnDialogueStart)
  (bind _output_get (Variables|Default|SetDialogueLines DialogueLines))
  (Utilities|Array|Add _output_get (Utilities|Struct|MakeDialogueLine "NAME" "DIALOGUE" 0 false true "NewEnumerator3" 0))
  (Variables|Default|SetCurrentDialogueLine 0)
  (bind _returnvalue_2 (UserInterface|CreateWidget "/Game/Blueprints/Dialogue/WBP_DialogueUI.WBP_DialogueUI_C" (Game|GetPlayerController 0) self))
  (bind _output_get_2 (Variables|Default|SetDialogueUI _returnvalue_2))
  (UserInterface|Viewport|AddtoViewport _output_get_2 0)
  (Pawn|Components|CharacterMovement|SetMovementMode (Variables|/Script/Engine.Character|GetCharacterMovement (Game|GetPlayerCharacter 0)) "MOVE_None" 0)
  (Input|SetInputModeUIOnly _returnvalue _output_get_2 "DoNotLock" false)
  (Variables|/Script/Engine.PlayerController|SetbShowMouseCursor _returnvalue true)
  (UserInterface|Animation|PlayAnimation (Variables|Default|GetDialogueUI) (Variables|/Game/Blueprints/Dialogue/WBP_DialogueUI.WBP_DialogueUI_C|GetStartDialogue (Variables|Default|GetDialogueUI)) 0.0 1 "Forward" 1.0 false)
  (CallFunction|DialogueContinue)
  (Utilities|FlowControl|Delay 1.05)
  (Variables|/Game/Blueprints/Dialogue/WBP_DialogueUI.WBP_DialogueUI_C|SetCanContinue (Variables|Default|GetDialogueUI) true))

(event Custom|DialogueContinue
  (if (not (.LastLine? (Utilities|Struct|BreakDialogueLine (Utilities|Array|Get(acopy) (Variables|Default|GetDialogueLines) (Variables|Default|GetCurrentDialogueLine)))))
    (Default|UpdateText (Variables|Default|GetDialogueUI) (Utilities|Array|Get(acopy) (Variables|Default|GetDialogueLines) (Variables|Default|GetCurrentDialogueLine)))
    (Math|Integer|IncrementInt (Variables|Default|GetCurrentDialogueLine))
    (else
      (CallFunction|DialogueEnd))))

(event Custom|DialogueEnd
  (bind _returnvalue (Game|GetPlayerController 0))
  (bind _dialogueui (Variables|Default|GetDialogueUI))
  (Variables|/Game/Blueprints/Dialogue/WBP_DialogueUI.WBP_DialogueUI_C|SetCanContinue (Variables|Default|GetDialogueUI) false)
  (Default|CallOnDialogueEnd)
  (UserInterface|Animation|PlayAnimation _dialogueui (Variables|/Game/Blueprints/Dialogue/WBP_DialogueUI.WBP_DialogueUI_C|GetEndDialogue _dialogueui) 0.0 1 "Forward" 1.0 false)
  (Utilities|FlowControl|Delay 1.05)
  (Widget|RemovefromParent _dialogueui)
  (Variables|Default|SetInDialogue? false)
  (Pawn|Components|CharacterMovement|SetMovementMode (Variables|/Script/Engine.Character|GetCharacterMovement (Game|GetPlayerCharacter 0)) "MOVE_Walking" 0)
  (Input|SetInputModeGameOnly _returnvalue true)
  (Variables|/Script/Engine.PlayerController|SetbShowMouseCursor _returnvalue false))

(event EventBeginPlay)

(fn ConstructionScript)