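; BP_Button is an interactable, lockable button that relays interactions to the actors it affects.
; Its Interact event reserves negative flags to lock, unlock or toggle the lock, while other flags press it.
; An unlocked press plays the use sound and sends BPI_Interaction's InteractMessage, with a per-index flag, to each implementing AffectedActor, marked as not called by the player.
; A locked press only plays the locked sound.
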(event EventBeginPlay)

(event EventInteract
  (params (Called%20By%20Player? :type Boolean) (Flag :type Integer))
  (switch int Flag
    (:Default
      (if (not (Variables|Default|GetLocked?)) :!label _label
        (Audio|PlaySoundatLocation (Variables|Default|GetUseSound) (Transformation|GetActorLocation) "0, 0, 0" 1.0 1.0 0.0 0 0 0 0)
        (for (_array_element _array_index) (Variables|Default|GetAffected%20Actors)
          (if (Utilities|DoesObjectImplementInterface _array_element "/Game/Blueprints/Interfaces/BPI_Interaction.BPI_Interaction_C")
            (Class|BPIInteraction|Interact(Message) _array_element false (Utilities|Array|Get(acopy) (Variables|Default|GetFlag) _array_index))))
        (else
          (Audio|PlaySoundatLocation (Variables|Default|GetLockedSound) (Transformation|GetActorLocation) "0, 0, 0" 1.0 1.0 0.0 0 0 0 0))))
    (:-3
      (bind _outputboolean (CallFunction|INVERTBoolean (Variables|Default|GetLocked?)))
      (Variables|Default|SetLocked? _outputboolean))
    (:-2
      (Variables|Default|SetLocked? false))
    (:-1
      (Variables|Default|SetLocked? true))
    (:0
      (goto _label))))

(fn ConstructionScript)