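; BP_TriggerOnce is a box trigger that calls TriggerEnter and TriggerExit at most once each for a BP_FirstPersonCharacter.
; Separate flags latch begin and end overlap, and are set before the character cast, so any overlapping actor can consume them.
; Both paths require the TriggerExit boolean, even entry, and an empty SpecificActorOnly, with no handling when that list is filled.
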(event OnComponentEndOverlap(BoxCollider)
  (params (OverlappedComponent :type Primitive%20Component%20Object%20Reference) (OtherActor :type Actor%20Object%20Reference) (OtherComp :type Primitive%20Component%20Object%20Reference) (OtherBodyIndex :type Integer))
  (if (not (Variables|Default|GetExitTriggered))
    (if (Variables|Default|GetTriggerExit?)
      (if (Utilities|Array|IsEmpty (Variables|Default|GetSpecificActorOnly))
        (Variables|Default|SetExitTriggered true)
        (Utilities|Casting|CastToBP_FirstPersonCharacter OtherActor)
        (CallFunction|TriggerExit)))))

(event OnComponentBeginOverlap(BoxCollider)
  (params (OverlappedComponent :type Primitive%20Component%20Object%20Reference) (OtherActor :type Actor%20Object%20Reference) (OtherComp :type Primitive%20Component%20Object%20Reference) (OtherBodyIndex :type Integer) (bFromSweep :type Boolean) (SweepResult :type Hit%20Result%20Structure%20%28by%20ref%29))
  (if (not (Variables|Default|GetEnterTriggered))
    (if (Variables|Default|GetTriggerExit?)
      (if (Utilities|Array|IsEmpty (Variables|Default|GetSpecificActorOnly))
        (Variables|Default|SetEnterTriggered true)
        (Utilities|Casting|CastToBP_FirstPersonCharacter OtherActor)
        (CallFunction|TriggerEnter)))))

(event EventBeginPlay
  (|CallParentFunction) ; This node is disabled and will not be called.\nDrag off pins to build functionality.
)

(fn ConstructionScript
  (|CallParentFunction))