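; BP_Keypad is an interactable code keypad that triggers linked actors when the correct code is entered.
; Interacting opens a WBP_KeypadUI widget with UI-only input and a visible cursor, and binds its TryUnlock event back to the keypad.
; A match against Code plays a success sound, fires OnSuccessUnlock and sends a BPI_Interaction Interact message to each compatible affected actor.
; A mismatch plays a failure sound and fires OnFailedUnlock.
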(event Custom|AttemptUnlock
  (params (Input :type Integer))
  (CallFunction|UnlockFunction Input))

(event EventInteract
  (bind _returnvalue (Game|GetPlayerController 0))
  (bind _returnvalue_2 (UserInterface|CreateWidget "/Game/Blueprints/Interaction/Widgets/WBP_KeypadUI.WBP_KeypadUI_C" (Game|GetPlayerController 0) self))
  (bind _output_get (Variables|Default|SetKeypadUI _returnvalue_2))
  (UserInterface|Viewport|AddtoViewport _output_get 0)
  (Input|SetInputModeUIOnly _returnvalue _returnvalue_2 "DoNotLock" true)
  (Variables|/Script/Engine.PlayerController|SetbShowMouseCursor _returnvalue true)
  (EventDispatchers|BindEventtoTryUnlock (Variables|Default|GetKeypadUI) (delegate Custom|AttemptUnlock)))

(fn ConstructionScript)

(fn UnlockFunction
  (params (Input :type Integer))
  (if (== Input (Variables|Default|GetCode))
    (Audio|PlaySound2D (Variables|Default|GetSuccessSound) 1.0 1.0 0.0 0 0)
    (Default|CallOnSuccessUnlock)
    (for _array_element (Variables|Default|GetAffectedActors)
      (if (Utilities|DoesObjectImplementInterface _array_element "/Game/Blueprints/Interfaces/BPI_Interaction.BPI_Interaction_C")
        (Class|BPIInteraction|Interact(Message) _array_element false)))
    (else
      (Audio|PlaySound2D (Variables|Default|GetFailedSound) 1.0 1.0 0.0 0 0)
      (Default|CallOnFailedUnlock))))