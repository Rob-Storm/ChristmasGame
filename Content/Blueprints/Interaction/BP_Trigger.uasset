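; BP_Trigger is a box trigger, sized at construction from ColliderDimensions, that sends interaction messages to configured actors on overlap.
; Enter and exit events each send paired flags through BPI_Interaction to their actor lists.
; Entry accepts the first-person character or actors in SpecificActorOnly; exit fires only for the character when that list is empty.
; Its own Interact event toggles, activates or deactivates the collider using negative flags.
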(event OnComponentBeginOverlap(BoxCollider)
  (params (OverlappedComponent :type Primitive%20Component%20Object%20Reference) (OtherActor :type Actor%20Object%20Reference) (OtherComp :type Primitive%20Component%20Object%20Reference) (OtherBodyIndex :type Integer) (bFromSweep :type Boolean) (SweepResult :type Hit%20Result%20Structure%20%28by%20ref%29))
  (if (Variables|Default|GetTriggerEnter?)
    (if (Utilities|Array|IsEmpty (Variables|Default|GetSpecificActorOnly))
      (Utilities|Casting|CastToBP_FirstPersonCharacter OtherActor)
      (CallFunction|TriggerEnter)
      (else
        (bind _compatible_ (CallFunction|CheckActorCompatibility OtherActor))
        (if _compatible_
          (CallFunction|TriggerEnter)
          (else
            (Development|PrintString "Collided Actor is not compatible with any index of SpecificActorOnly")))))))

(event OnComponentEndOverlap(BoxCollider)
  (params (OverlappedComponent :type Primitive%20Component%20Object%20Reference) (OtherActor :type Actor%20Object%20Reference) (OtherComp :type Primitive%20Component%20Object%20Reference) (OtherBodyIndex :type Integer))
  (if (Variables|Default|GetTriggerExit?)
    (if (Utilities|Array|IsEmpty (Variables|Default|GetSpecificActorOnly))
      (Utilities|Casting|CastToBP_FirstPersonCharacter OtherActor)
      (CallFunction|TriggerExit))))

(event Custom|TriggerExit
  (for (_array_element _array_index) (Variables|Default|GetExitAffectedActors)
    (if (Utilities|DoesObjectImplementInterface _array_element "/Game/Blueprints/Interfaces/BPI_Interaction.BPI_Interaction_C")
      (Class|BPIInteraction|Interact(Message) _array_element false (Utilities|Array|Get(acopy) (Variables|Default|GetExitFlags) _array_index))
      (else
        (Development|PrintString "Affect Actor(s) do not implement BPI_Interaction!")))))

(event Custom|TriggerEnter
  (for (_array_element _array_index) (Variables|Default|GetEnterAffectedActors)
    (if (Utilities|DoesObjectImplementInterface _array_element "/Game/Blueprints/Interfaces/BPI_Interaction.BPI_Interaction_C")
      (Class|BPIInteraction|Interact(Message) _array_element false (Utilities|Array|Get(acopy) (Variables|Default|GetEnterFlags) _array_index))
      (else
        (Development|PrintString "Affect Actor(s) do not implement BPI_Interaction!")))))

(event EventBeginPlay)

(event EventInteract
  (params (Called%20By%20Player? :type Boolean) (Flag :type Integer))
  (bind _boxcollider (Variables|Default|GetBoxCollider))
  (bind _boxcollider_2 (Variables|Default|GetBoxCollider))
  (switch int Flag
    (:-3
      (bind _outputboolean (CallFunction|INVERTBoolean (Components|Activation|IsActive _boxcollider)))
      (Components|Activation|SetActive _boxcollider _outputboolean false))
    (:-2
      (Components|Activation|SetActive _boxcollider_2 true false))
    (:-1
      (Components|Activation|SetActive _boxcollider_2 false false))))

(fn ConstructionScript
  (Components|Box|SetBoxExtent (Variables|Default|GetBoxCollider) (Variables|Default|GetColliderDimensions) true))

(fn CheckActorCompatibility
  (params (Actor :type Actor%20Object%20Reference))
  (bind _array_element (Utilities|Array|ForEachLoopwithBreak (Variables|Default|GetSpecificActorOnly) :!label _label)
    (:LoopBody
      (if (== _array_element Actor)
        (goto _label Break)))
    (:Completed
      (return (== _array_element Actor)))))