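; BP_Character is a character Blueprint that starts its own dialogue when interacted with.
; On BeginPlay it finds and caches the first BP_DialogueManager in the level, printing an error if none exists.
; Its Interact event passes the Dialogue data to that manager's DialogueStart, but only when the data is not empty.
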(event EventBeginPlay
  (bind _outactors (Actor|GetAllActorsOfClass "/Game/Blueprints/Dialogue/BP_DialogueManager.BP_DialogueManager_C"))
  (Utilities|IsValid (Utilities|Array|Get(acopy) _outactors)
    (:Is%20Valid
      (Variables|Default|SetDialogueManager (Utilities|Array|Get(acopy) _outactors)))
    (:Is%20Not%20Valid
      (Development|PrintString "Error! No BP_DialogueManager in level!" true true "(R=1.000000,G=0.000000,B=0.000000,A=1.000000)" 5.0))))

(event EventInteract
  (params (Called%20By%20Player? :type Boolean) (Flag :type Integer))
  (if (> (Utilities|Array|Length (Variables|Default|GetDialogue)) 0)
    (Default|DialogueStart (Variables|Default|GetDialogueManager) (Variables|Default|GetDialogue))))

(fn ConstructionScript)