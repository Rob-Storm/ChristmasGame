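; BP_Door is a door that tracks open and locked state, starting open or closed according to StartsOpen.
; Interact uses an integer Flag: negative codes set or flip Locked and PlayerNoInteract, while others toggle the door or play a locked sound.
; ToggleDoor plays a sound and calls OpenDoor or CloseDoor, which only set Open here.
; The check blocking player interaction through PlayerNoInteract is unwired, so it has no effect.
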(event Custom|Toggle%20Door
  (if (Variables|Default|GetOpen?)
    (Audio|PlaySoundatLocation (Variables|Default|GetClosedSound) (Transformation|GetActorLocation) "0, 0, 0" 1.0 1.0 0.0 0 0 0 0)
    (CallFunction|CloseDoor)
    (else
      (Audio|PlaySoundatLocation (Variables|Default|GetOpenSound) (Transformation|GetActorLocation) "0, 0, 0" 1.0 1.0 0.0 0 0 0 0)
      (CallFunction|OpenDoor))))

(event Custom|OpenDoor
  (Variables|Default|SetOpen? true))

(event Custom|CloseDoor
  (Variables|Default|SetOpen? false))

(event EventBeginPlay
  (if (Variables|Default|GetStartsOpen?)
    (CallFunction|OpenDoor)
    (else
      (CallFunction|CloseDoor))))

(event EventInteract
  (params (Called%20By%20Player? :type Boolean) (Flag :type Integer))
  (switch int Flag
    (:Default
      (if (not (Variables|Default|GetLocked?)) :!label _label
        (CallFunction|ToggleDoor)
        (else
          (Audio|PlaySoundatLocation (Variables|Default|GetLockedSound) (Transformation|GetActorLocation) "0, 0, 0" 1.0 1.0 0.0 0 0 0 0))))
    (:-6
      (bind _outputboolean (CallFunction|InvertBoolean (Variables|Default|GetPlayerNoInteract?)))
      (Variables|Default|SetPlayerNoInteract? _outputboolean))
    (:-5
      (Variables|Default|SetPlayerNoInteract? false))
    (:-4
      (Variables|Default|SetPlayerNoInteract? true))
    (:-3
      (bind _outputboolean_2 (CallFunction|InvertBoolean (Variables|Default|GetLocked?)))
      (Variables|Default|SetLocked? _outputboolean_2))
    (:-2
      (Variables|Default|SetLocked? true))
    (:-1
      (Variables|Default|SetLocked? false))
    (:0
      (goto _label))))

(fn ConstructionScript)