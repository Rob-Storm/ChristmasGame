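; BP_DoorMoving is a door variant that opens and closes by relocating the whole actor between two positions.
; BeginPlay records the starting location as ClosePosition, while OpenPosition is read from a variable this graph never sets.
; OpenDoor and CloseDoor call the parent, then snap instantly to their position without sweep or interpolation.
; Interact and ToggleDoor only forward to the parent class.
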(event EventBeginPlay
  (Variables|Default|SetClosePosition (Transformation|GetActorLocation))
  (|CallParentFunction))

(event EventInteract
  (params (Called%20By%20Player? :type Boolean) (Flag :type Integer))
  (|CallParentFunction Called%20By%20Player? Flag))

(event EventCloseDoor
  (|CallParentFunction)
  (Transformation|SetActorLocation (Variables|Default|GetClosePosition) false false))

(event EventOpenDoor
  (|CallParentFunction)
  (Transformation|SetActorLocation (Variables|Default|GetOpenPosition) false false))

(event EventToggleDoor
  (|CallParentFunction))

(fn ConstructionScript)