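; BP_DoorRotating is an interactable door that toggles between open and closed when Interact fires.
; On BeginPlay it caches the actor rotation as the closed rotation and applies the initial state from StartsOpen.
; Toggling snaps the Hinge component instantly to the open or closed world rotation, with no interpolation, and plays the matching sound at the door's location.
; OpenRotation is absolute in world space rather than relative to the placed door.
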(event Custom|ToggleDoor
  (if (Variables|Default|GetOpen?)
    (CallFunction|CloseDoor)
    (else
      (CallFunction|OpenDoor))))

(event Custom|OpenDoor
  (Variables|Default|SetOpen? true)
  (Transformation|SetWorldRotation (Variables|Default|GetHinge) (Variables|Default|GetOpenRotation) false false)
  (Audio|PlaySoundatLocation (Variables|Default|GetOpenSound) (Transformation|GetActorLocation) "0, 0, 0" 1.0 1.0 0.0 0 0 0 0))

(event Custom|CloseDoor
  (Variables|Default|SetOpen? false)
  (Transformation|SetWorldRotation (Variables|Default|GetHinge) (Variables|Default|GetCloseRotation) false false)
  (Audio|PlaySoundatLocation (Variables|Default|GetCloseSound) (Transformation|GetActorLocation) "0, 0, 0" 1.0 1.0 0.0 0 0 0 0))

(event EventBeginPlay
  (Variables|Default|SetCloseRotation (Transformation|GetActorRotation))
  (if (Variables|Default|GetStartsOpen?)
    (Variables|Default|SetOpen? true)
    (Transformation|SetWorldRotation (Variables|Default|GetHinge) (Variables|Default|GetOpenRotation) false false)
    (else
      (Variables|Default|SetOpen? false)
      (Transformation|SetWorldRotation (Variables|Default|GetHinge) (Variables|Default|GetCloseRotation) false false))))

(event EventInteract
  (CallFunction|ToggleDoor))

(fn ConstructionScript)