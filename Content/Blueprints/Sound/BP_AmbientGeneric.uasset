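; Generic placeable sound actor that plays a configurable sound on BeginPlay when PlayOnAwake is set, or through its events.
; The construction script applies sound, volume and pitch to the AudioComponent.
; Interact uses its Flag to toggle, stop after a delay, or by default play from StartTime.
; PlaySound switches attenuation to SA_None for 2D sounds, a step the BeginPlay autoplay skips.
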(event Custom|PlaySound
  (bind _audiocomponent (Variables|Default|GetAudioComponent))
  (bind _start_time (Variables|Default|GetStart%20Time))
  (if (Variables|Default|Get2DSound?)
    (Variables|/Script/Engine.AudioComponent|SetAttenuationSettings _audiocomponent "/Game/Sound/SA_None.SA_None")
    (Audio|Components|Audio|Play _audiocomponent _start_time)
    (else
      (Audio|Components|Audio|Play _audiocomponent _start_time))))

(event EventBeginPlay
  (if (Variables|Default|GetPlayOnAwake?)
    (Audio|Components|Audio|Play (Variables|Default|GetAudioComponent) (Variables|Default|GetStart%20Time))))

(event EventInteract
  (params (Called%20By%20Player? :type Boolean) (Flag :type Integer))
  (bind _audiocomponent (Variables|Default|GetAudioComponent))
  (switch int Flag
    (:Default
      (CallFunction|PlaySound :!label _label))
    (:-2
      (if (Audio|Components|Audio|IsPlaying _audiocomponent)
        (Audio|Components|Audio|StopDelayed _audiocomponent (Variables|Default|GetStop%20Time))
        (else
          (CallFunction|PlaySound))))
    (:-1
      (Audio|Components|Audio|StopDelayed _audiocomponent (Variables|Default|GetStop%20Time)))
    (:0
      (goto _label))))

(fn ConstructionScript
  (bind _audiocomponent (Variables|Default|GetAudioComponent))
  (Audio|Components|Audio|SetSound _audiocomponent (Variables|Default|GetSound))
  (Audio|Components|Audio|SetVolumeMultiplier _audiocomponent (Variables|Default|GetVolumeMultiplier) :!class /Script/Engine.AudioComponent)
  (Audio|Components|Audio|SetPitchMultiplier _audiocomponent (Variables|Default|GetPitchMultiplier)))