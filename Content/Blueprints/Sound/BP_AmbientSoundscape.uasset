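; BP_AmbientSoundscape is a placed actor that plays an ambient sound, with only one soundscape intended to be active at a time.
; The construction script assigns the sound, and BeginPlay stops playback, fading it in only if this instance is flagged as default.
; Interact triggers ChangeSoundscape, which fades out every BP_AmbientSoundscape in the level, itself included, then fades this one in to its configured volume.
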(event Custom|ChangeSoundscape
  (bind _outactors (Actor|GetAllActorsOfClass "BP_AmbientSoundscape_C"))
  (if (Utilities|Array|IsNotEmpty _outactors)
    (for _array_element _outactors
      (CallFunction|StopSoundscape _array_element))
    (CallFunction|StartSoundscape)))

(event Custom|StopSoundscape
  (Audio|Components|Audio|FadeOut (Variables|Default|GetAudioComponent) (Variables|Default|GetFadeOutDuration) 0.0 "Linear" :!class /Script/Engine.AudioComponent))

(event Custom|StartSoundscape
  (Audio|Components|Audio|FadeIn (Variables|Default|GetAudioComponent) (Variables|Default|GetFadeInDuration) (Variables|Default|GetSoundScapeVolume) 0.0 "Linear" :!class /Script/Engine.AudioComponent))

(event EventInteract
  (params (Called%20By%20Player? :type Boolean) (Flag :type Integer))
  (CallFunction|ChangeSoundscape))

(event EventBeginPlay
  (Audio|Components|Audio|Stop (Variables|Default|GetAudioComponent))
  (if (Variables|Default|GetDefaultSoundscape?)
    (CallFunction|StartSoundscape)))

(fn ConstructionScript
  (Audio|Components|Audio|SetSound (Variables|Default|GetAudioComponent) (Variables|Default|GetSound)))